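; OSC receiver Blueprint that drives a raymarched post-process visual of a motion-capture skeleton and scene objects.
; A local OSC server routes /vis messages to material parameters and /mocap messages to filtered, rotation-corrected joints, from which edges are built.
; Joint and edge matrices, plus object settings, are drawn texel by texel into float render targets that the raymarching material reads.
; It also spawns debug actors that follow the skeleton.
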(event `self.ReceiveBeginPlay`
  ;[0.4913 0.8525 1 1 110] OSC HANDLER
  (`|ExecutionSequence`
    (:`then_0`
      ;[0.7723 0.5645 1 1 95] MATERIAL AND TEXTURE BUFFER CREATION
      (bind _returnvalue (`KismetMaterialLibrary.CreateDynamicMaterialInstance` "/Game/Pedro/Material/RaymarchingShaders/Raymarching_GroundRipple.Raymarching_GroundRipple"))
      (bind _output_get (set `self.RaymarchingMat` _returnvalue))
      (bind _returnvalue_2 (`GameplayStatics.GetActorOfClass` "/Script/Engine.PostProcessVolume"))
      (set `PostProcessVolume.Settings` (make `PostProcessSettings` :`WeightedBlendables` (make `WeightedBlendables` (`|MakeArray` (make `WeightedBlendable` 1.0 _output_get)))) _returnvalue_2)
      (bind _returnvalue_3 (`KismetRenderingLibrary.CreateRenderTarget2D` 4 23 "RTF_RGBA32f"))
      (bind _returnvalue_4 (`KismetRenderingLibrary.CreateRenderTarget2D` 4 20 "RTF_RGBA32f"))
      (bind _returnvalue_5 (`KismetRenderingLibrary.CreateRenderTarget2D` 34 2 "RTF_R32f"))
      (set `self.JointTextureRenderTarget` _returnvalue_3)
      (set `self.EdgeTextureRenderTarget` _returnvalue_4)
      (set `self.ObjectTextureRenderTarget` _returnvalue_5)
      (`KismetArrayLibrary.Array_Set` (`self.objects`) 0 (make `/Game/Pedro/MyObjects` (`KismetMathLibrary.MakeTransform` (0.0 0.0 0.0)) 0 0.5 0.3 (0.1 0.1 0.1) (0.1 0.1 0.1) (0.1 0.1 0.1) (make `Color` 1) 0.5 0.5 0.0 10.0 0.5 0.1))
      (`KismetArrayLibrary.Array_Set` (`self.objects`) 1 (make `/Game/Pedro/MyObjects` (`KismetMathLibrary.MakeTransform` (0.0 0.0 10.0)) 1 0.1 0.8 (0.1 0.1 0.1) (0.1 0.1 0.1) (0.1 0.1 0.1) (make `Color` 0 1) 0.5 0.5 0.0 20.0 0.5 0.1)))
    (:`then_1`
      (bind _returnvalue_6 (`OSCManager.CreateOSCServer` "127.0.0.1" 9005 false true "OSC_Server" null))
      (bind _output_get_2 (set `self.OSC Server` _returnvalue_6))
      (add `OSCServer.OnOscMessageReceived` _output_get_2 (delegate `MessageReceived`)))))

(event `MessageReceived`
  (params (Message :type "OSCMessage Structure (by ref)") (IPAddress :type String) (Port :type Integer))
  ;[0.4913 0.8525 1 1 110] OSC HANDLER
  ;;[1 1 1] OSC CONTROLLER
  (set `self.Message` Message)
  (bind _returnvalue (`OSCManager.GetOSCMessageAddress` Message))
  (bind _returnvalue_2 (`OSCManager.GetOSCAddressFullPath` _returnvalue))
  (switch `string` _returnvalue_2
    (:`Default`
      (`self.DefaultStatement` _returnvalue :!label _label))
    (:`/mocap/joint/pos_world`
      ;;[1 1 1] MOCAP
      (bind _values (`OSCManager.GetAllFloats` Message))
      (bind _vectors (`self.ConvertFloatArrayToPositionVector` _values)))
    (:`/mocap/joint/rot_world`
      (bind _values_2 (`OSCManager.GetAllFloats` Message))
      (bind _vectors_2 (`self.ConvertFloatArrayToRotator` _values_2))
      (if (and (`KismetArrayLibrary.Array_IsNotEmpty` _vectors) (`KismetArrayLibrary.Array_IsNotEmpty` _vectors_2))
        (set `self.Positions` _vectors)
        (set `self.Rotations` _vectors_2)
        (`self.Update Edges`)
        (`self.DrawTexture`)))
    (:`/vis/bgcolor`
      ;;[1 1 1] COLORS
      (bind _values_3 (`OSCManager.GetAllFloats` Message))
      (`self.SetMaterialColorParameter` _values_3 "bgColor"))
    (:`/vis/objectcolor`
      (bind _values_4 (`OSCManager.GetAllFloats` Message))
      (`self.SetMaterialColorParameter` _values_4 "objectColor"))
    (:`/vis/lightposition`
      ;;[1 1 1] LIGHT
      (bind _values_5 (`OSCManager.GetAllFloats` Message))
      (`self.SetMaterialColorParameter` _values_5 "lightPosition"))
    (:`/vis/lightambientscale`
      (bind _values_6 (`OSCManager.GetAllFloats` Message))
      (`self.Set Material Float` _values_6 "lightAmbientScale"))
    (:`/vis/lightdiffusescale`
      (bind _values_7 (`OSCManager.GetAllFloats` Message))
      (`self.Set Material Float` _values_7 "lightDiffuseScale"))
    (:`/vis/lightspecularscale`
      (bind _values_8 (`OSCManager.GetAllFloats` Message))
      (`self.Set Material Float` _values_8 "lightSpecularScale"))
    (:`/vis/lightspecularpow`
      (bind _values_9 (`OSCManager.GetAllFloats` Message))
      (`self.Set Material Float` _values_9 "lightSpecularPow"))
    (:`/vis/lightocclusionscale`
      ;;[1 1 1] AMBIENT OCCLUSION
      (bind _values_10 (`OSCManager.GetAllFloats` Message))
      (`self.Set Material Float` _values_10 "lightOcclusionScale"))
    (:`/vis/lightocclusionrange`
      (bind _values_11 (`OSCManager.GetAllFloats` Message))
      (`self.Set Material Float` _values_11 "lightOcclusionRange"))
    (:`/vis/lightocclusionresolution`
      (bind _values_12 (`OSCManager.GetAllFloats` Message))
      (`self.Set Material Float` _values_12 "lightOcclusionResolution"))
    (:`/vis/jointprimitive`
      ;;[1 1 1] JOINTS
      (bind _value (`OSCManager.GetInt32` Message))
      (`MaterialInstanceDynamic.SetScalarParameterValue` (`self.RaymarchingMat`) "jointPrimitive" (`KismetMathLibrary.Conv_IntToDouble` _value)))
    (:`/vis/jointsize`
      (bind _values_13 (`OSCManager.GetAllFloats` Message))
      (`MaterialInstanceDynamic.SetVectorParameterValue` (`self.RaymarchingMat`) "jointSize" (`KismetMathLibrary.MakeColor` (* (`|GetArrayItem` _values_13) 10.0) (* (`|GetArrayItem` _values_13 1) 10.0) (* (`|GetArrayItem` _values_13 2) 10.0))))
    (:`/vis/jointround`
      (bind _values_14 (`OSCManager.GetAllFloats` Message))
      (`self.Set Material Float` _values_14 "jointRound"))
    (:`/vis/jointsmooth`
      (bind _values_15 (`OSCManager.GetAllFloats` Message))
      (`self.Set Material Float` _values_15 "jointSmooth"))
    (:`/vis/edgeprimitive`
      ;;[1 1 1] EDGES
      (bind _value_2 (`OSCManager.GetInt32` Message))
      (`MaterialInstanceDynamic.SetScalarParameterValue` (`self.RaymarchingMat`) "edgePrimitive" (`KismetMathLibrary.Conv_IntToDouble` _value_2)))
    (:`/vis/edgesize`
      (bind _values_16 (`OSCManager.GetAllFloats` Message))
      (set `self.edgeScale` (`KismetMathLibrary.MakeVector` (* (`|GetArrayItem` _values_16) 10.0) (* (`|GetArrayItem` _values_16 1) 10.0) (* (`|GetArrayItem` _values_16 2) 1.0))))
    (:`/vis/edgeround`
      (bind _values_17 (`OSCManager.GetAllFloats` Message))
      (`self.Set Material Float` _values_17 "edgeRound"))
    (:`/vis/edgesmooth`
      (bind _values_18 (`OSCManager.GetAllFloats` Message))
      (`self.Set Material Float` _values_18 "edgeSmooth"))
    (:`/vis/jointedgesmooth`
      (bind _values_19 (`OSCManager.GetAllFloats` Message))
      (`self.Set Material Float` _values_19 "jointEdgeSmoothing"))
    (:`/vis/groundprimitive`
      ;;[1 1 1] OBJECT
      (bind _value_3 (`OSCManager.GetInt32` Message))
      (`MaterialInstanceDynamic.SetScalarParameterValue` (`self.RaymarchingMat`) "groundPrimitive" (`KismetMathLibrary.Conv_IntToDouble` _value_3)))
    (:`/vis/groundposition`
      (bind _values_20 (`OSCManager.GetAllFloats` Message))
      (`self.SetMaterialColorParameter` _values_20 "groundPosition"))
    (:`/vis/groundrotation`
      (goto _label))
    (:`/vis/groundsize`
      (bind _values_21 (`OSCManager.GetAllFloats` Message))
      (`self.SetMaterialColorParameter` _values_21 "groundSize"))
    (:`/vis/groundround`
      (bind _values_22 (`OSCManager.GetAllFloats` Message))
      (`self.Set Material Float` _values_22 "groundRound"))
    (:`/vis/groundsmooth`
      (bind _values_23 (`OSCManager.GetAllFloats` Message))
      (`self.Set Material Float` _values_23 "groundSmooth"))))

(event `Update Edges`
  (bind _positions (`self.Positions`))
  (bind _positions_2 (`self.Positions`))
  ;[1 1 1 1 63] HANDLING Edges
  (`|ExecutionSequence`
    (:`then_0`
      (`/Engine/EditorBlueprintResources/StandardMacros.DoOnce` false
        (:`Completed`
          (`self.CreateEdges`))))
    (:`then_1`
      (for (_array_element _array_index) (`self.edges`)
        (bind (_transform _length _parent _child) (break `/Game/Pedro/MyEdges` _array_element))
        (bind (_x _y _z _w) (`KismetMathLibrary.BreakVector4` (`|GetArrayItem` (`self.Rotations`) _parent)))
        (`KismetArrayLibrary.Array_Set` (`self.edges`) _array_index (make `/Game/Pedro/MyEdges` (`KismetMathLibrary.MakeTransform` (/ (+ (`|GetArrayItem` _positions_2 _parent) (`|GetArrayItem` _positions_2 _child)) 2) (`KismetMathLibrary.Quat_Rotator` (`KismetMathLibrary.MakeQuat` _x _y _z _w)) (.scale _transform)) (/ (`KismetMathLibrary.VSize` (- (`|GetArrayItem` _positions _child) (`|GetArrayItem` _positions _parent))) 10.0) _parent _child))))
    (:`then_2`
      (`self.DebugWithStandarSkeleton`))))

(event `DrawTexture`
  (bind _raymarchingmat (`self.RaymarchingMat`))
  (bind (_edgescale_x _edgescale_y _edgescale_z) (`KismetMathLibrary.BreakVector` (`self.edgeScale`)))
  ;[1 1 1 1 110] DRAWING PARAMETER TEXTURE
  (`|ExecutionSequence`
    (:`then_0`
      (bind (_canvas _size _context) (`KismetRenderingLibrary.BeginDrawCanvasToRenderTarget` (`self.JointTextureRenderTarget`)))
      ;;[0.6746 1 0.669] JOINTS
      (for (_array_element _array_index) (`self.Positions`)
        (for _index (range 4)
          (bind (_x _y _z _w) (`KismetMathLibrary.BreakVector4` (`|GetArrayItem` (`self.Rotations`) _array_index)))
          ;;;[1 1 1] C++ FUNCTION
          (bind _returnvalue (`self.CreateMatrixFromPositionRotationScale` _array_element (`KismetMathLibrary.Quat_Normalized` (`KismetMathLibrary.MakeQuat` _x _y _z _w)) (`KismetMathLibrary.Vector_One`)))
          (bind _returnvalue_2 (`self.GetColumnFromMatrix` _returnvalue _index))
          (bind (_x_2 _y_2 _z_2 _w_2) (`KismetMathLibrary.BreakVector4` _returnvalue_2))
          (`Canvas.K2_DrawTexture` _canvas null (`KismetMathLibrary.MakeVector2D` (`KismetMathLibrary.Conv_IntToDouble` _index) (`KismetMathLibrary.Conv_IntToDouble` _array_index)) (1.0 1.0) (0.0 0.0) (1.0 1.0) (`KismetMathLibrary.MakeColor` _x_2 _y_2 _z_2 _w_2) "BLEND_Masked" 0.0 (0.5 0.5))))
      ;;;[0.9539 1 0.9858] Set PARAMETERS IN MATERIAL
      (`KismetRenderingLibrary.EndDrawCanvasToRenderTarget` _context)
      (`MaterialInstanceDynamic.SetTextureParameterValue` _raymarchingmat "jointTransformTexture" (`self.JointTextureRenderTarget`))
      (`MaterialInstanceDynamic.SetScalarParameterValue` _raymarchingmat "jointCount" (`KismetMathLibrary.Conv_IntToDouble` (`KismetArrayLibrary.Array_Length` (`self.Positions`)))))
    (:`then_1`
      (bind (_canvas_2 _size_2 _context_2) (`KismetRenderingLibrary.BeginDrawCanvasToRenderTarget` (`self.EdgeTextureRenderTarget`)))
      ;;[1 0.3729 0.343] EDGES
      (for (_array_element_2 _array_index_2) (`self.edges`)
        (for _index_2 (range 4)
          (bind (_transform _length) (break `/Game/Pedro/MyEdges` _array_element_2))
          ;;;[1 1 1] C++ FUNCTION
          (bind _returnvalue_3 (`self.CreateMatrixFromPositionRotationScale` (.location _transform) (`KismetMathLibrary.Quat_Normalized` (`KismetMathLibrary.Conv_RotatorToQuaternion` (.rotation _transform))) (`KismetMathLibrary.MakeVector` _edgescale_x _edgescale_y (* (* _length 10.0) _edgescale_z))))
          (bind _returnvalue_4 (`self.GetColumnFromMatrix` _returnvalue_3 _index_2))
          (bind (_x_3 _y_3 _z_3 _w_3) (`KismetMathLibrary.BreakVector4` _returnvalue_4))
          (`Canvas.K2_DrawTexture` _canvas_2 null (`KismetMathLibrary.MakeVector2D` (`KismetMathLibrary.Conv_IntToDouble` _index_2) (`KismetMathLibrary.Conv_IntToDouble` _array_index_2)) (1.0 1.0) (0.0 0.0) (1.0 1.0) (`KismetMathLibrary.MakeColor` _x_3 _y_3 _z_3 _w_3) "BLEND_Masked" 0.0 (0.5 0.5))))
      ;;;[0.9539 1 0.9858] Set PARAMETERS IN MATERIAL
      (`KismetRenderingLibrary.EndDrawCanvasToRenderTarget` _context_2)
      (`MaterialInstanceDynamic.SetTextureParameterValue` (`self.RaymarchingMat`) "edgeTransformTexture" (`self.EdgeTextureRenderTarget`)))
    (:`then_2`
      (bind (_canvas_3 _size_3 _context_3) (`KismetRenderingLibrary.BeginDrawCanvasToRenderTarget` (`self.ObjectTextureRenderTarget`)))
      (for (_array_element_3 _array_index_3) (`self.objects`)
        (bind (_transform_2 _primitive _rounding _smoothing _frequencies _amplitude _phase _color _ambientscale _diffusescale _specularscale _specularpow _occlusionscale _occlusionrange) (break `/Game/Pedro/MyObjects` _array_element_3))
        (bind _returnvalue_5 (`self.CreateMatrixFromPositionRotationScale` (.location _transform_2) (`KismetMathLibrary.Conv_RotatorToQuaternion` (.rotation _transform_2)) (.scale _transform_2)))
        (for (_array_element_4 _array_index_4) (`|MakeArray` (`.X` (break `Plane` (break `Matrix` _returnvalue_5))) (`.Y` (break `Plane` (break `Matrix` _returnvalue_5))) (`.Z` (break `Plane` (break `Matrix` _returnvalue_5))) (break `Plane` (break `Matrix` _returnvalue_5)) (`.X` (break `Plane` (`.YPlane` (break `Matrix` _returnvalue_5)))) (`.Y` (break `Plane` (`.YPlane` (break `Matrix` _returnvalue_5)))) (`.Z` (break `Plane` (`.YPlane` (break `Matrix` _returnvalue_5)))) (break `Plane` (`.YPlane` (break `Matrix` _returnvalue_5))) (`.X` (break `Plane` (`.ZPlane` (break `Matrix` _returnvalue_5)))) (`.Y` (break `Plane` (`.ZPlane` (break `Matrix` _returnvalue_5)))) (`.Z` (break `Plane` (`.ZPlane` (break `Matrix` _returnvalue_5)))) (break `Plane` (`.ZPlane` (break `Matrix` _returnvalue_5))) (`.X` (break `Plane` (`.WPlane` (break `Matrix` _returnvalue_5)))) (`.Y` (break `Plane` (`.WPlane` (break `Matrix` _returnvalue_5)))) (`.Z` (break `Plane` (`.WPlane` (break `Matrix` _returnvalue_5)))) (break `Plane` (`.WPlane` (break `Matrix` _returnvalue_5))) (`KismetMathLibrary.Conv_IntToDouble` _primitive) _rounding _smoothing (.x _frequencies) (.y _frequencies) (.z _frequencies) (.x _amplitude) (.y _amplitude) (.z _amplitude) (.x _phase) (.y _phase) (.z _phase) (`KismetMathLibrary.Conv_ByteToDouble` (break `Color` _color)) (`KismetMathLibrary.Conv_ByteToDouble` (`.G` (break `Color` _color))) (`KismetMathLibrary.Conv_ByteToDouble` (`.R` (break `Color` _color))) _ambientscale _diffusescale _specularscale _specularpow _occlusionscale _occlusionrange)
          (`Canvas.K2_DrawTexture` _canvas_3 null (`KismetMathLibrary.MakeVector2D` (`KismetMathLibrary.Conv_IntToDouble` _array_index_4) (`KismetMathLibrary.Conv_IntToDouble` _array_index_3)) (1.0 1.0) (0.0 0.0) (1.0 1.0) (`KismetMathLibrary.MakeColor` _array_element_4) "BLEND_Masked" 0.0 (0.5 0.5))))
      (`KismetRenderingLibrary.EndDrawCanvasToRenderTarget` _context_3)
      (`MaterialInstanceDynamic.SetTextureParameterValue` (`self.RaymarchingMat`) "ObjectParameterTexture" (`self.ObjectTextureRenderTarget`)))))

(event `DebugWithStandarSkeleton`
  ;[0.6986 0 1 1 110] DEBUG!
  (`|ExecutionSequence`
    (:`then_0`
      (`/Engine/EditorBlueprintResources/StandardMacros.DoOnce` false
        (:`Completed`
          (for (_array_element _array_index) (`self.Positions`)
            (bind _returnvalue (`|SpawnActorFromClass` "/Game/Pedro/Blueprints/DebugClass.DebugClass_C" (`KismetMathLibrary.MakeTransform` _array_element (struct) (0.5 0.5 0.5)) "Undefined" "MultiplyWithRoot" null null))
            (`KismetArrayLibrary.Array_Set` (`self.JointDebug`) _array_index _returnvalue true))
          (for _array_element_2 (`self.edges`)
            (bind (_transform _length) (break `/Game/Pedro/MyEdges` _array_element_2))
            (bind _returnvalue_2 (`|SpawnActorFromClass` "/Game/Pedro/Blueprints/DebugClass.DebugClass_C" (`KismetMathLibrary.MakeTransform` (.location _transform) (.rotation _transform) (`KismetMathLibrary.MakeVector` 0.2 0.2 _length)) "Undefined" "MultiplyWithRoot" null null))
            (`PrimitiveComponent.SetMaterial` (`/Game/Pedro/Blueprints/DebugClass.Cube` _returnvalue_2) 0 "/Game/LevelPrototyping/Materials/MI_Solid_Blue.MI_Solid_Blue")
            (`KismetArrayLibrary.Array_Add` (`self.EdgesDebug`) _returnvalue_2)))))
    (:`then_1`
      (for (_array_element_3 _array_index_2) (`self.JointDebug`)
        (`self.K2_SetActorLocation` _array_element_3 (`|GetArrayItem` (`self.Positions`) _array_index_2) false false)
        (bind (_x _y _z _w) (`KismetMathLibrary.BreakVector4` (`|GetArrayItem` (`self.Rotations`) _array_index_2)))
        (`self.K2_SetActorRotation` _array_element_3 (`KismetMathLibrary.Quat_Rotator` (`KismetMathLibrary.MakeQuat` _x _y _z _w)) false)
        (for (_array_element_4 _array_index_3) (`self.EdgesDebug`)
          (bind (_transform_2 _length_2) (break `/Game/Pedro/MyEdges` (`|GetArrayItem` (`self.edges`) _array_index_3)))
          (`self.K2_SetActorLocation` _array_element_4 (.location _transform_2) false false)
          (`self.K2_SetActorRotation` _array_element_4 (.rotation _transform_2) false)
          (`self.SetActorScale3D` _array_element_4 (`KismetMathLibrary.MakeVector` 0.2 0.2 _length_2)))))))

(fn `Adapt RotationsBlueprint`
  (params (Rotations :type "Vector4 Structure") (counter :type Integer))
  (returns (RotationsAdapted :type "Vector4 Structure"))
  (locals (rotationChange :type "Rotator Structure"))
  (bind (_x _y _z _w) (`KismetMathLibrary.BreakVector4` Rotations))
  (bind (_x_2 _y_2 _z_2 _w_2) (`KismetMathLibrary.BreakQuat` (* (`KismetMathLibrary.MakeQuat` _x _y _z _w) (`KismetMathLibrary.Conv_RotatorToQuaternion` (`local.rotationChange`)))))
  (switch `int` counter
    (:`Default`
      (set `local.rotationChange` (struct :`Roll` 180.0) :!label _label))
    (:`0`
      (set `local.rotationChange` (struct) :!label _label_2))
    (:`1`
      (goto _label))
    (:`2`
      (goto _label))
    (:`3`
      (set `local.rotationChange` (struct :`Roll` -90.0) :!label _label_3))
    (:`4`
      (goto _label_3))
    (:`5`
      (goto _label))
    (:`6`
      (goto _label))
    (:`7`
      (goto _label_3))
    (:`8`
      (goto _label_3))
    (:`9`
      (goto _label_2))
    (:`10`
      (goto _label_2))
    (:`11`
      (goto _label_2))
    (:`12`
      (goto _label_2))
    (:`13`
      (set `local.rotationChange` (struct :`Pitch` -90.0) :!label _label_4))
    (:`14`
      (goto _label_4))
    (:`15`
      (goto _label_4))
    (:`16`
      (goto _label_4))
    (:`17`
      (set `local.rotationChange` (struct :`Pitch` 90.0) :!label _label_5))
    (:`18`
      (goto _label_5))
    (:`19`
      (goto _label_5))
    (:`20`
      (goto _label_5))
    (:`21`
      (goto _label_2))
    (:`22`
      (goto _label_2)))
  (return (`KismetMathLibrary.MakeVector4` _x_2 _y_2 _z_2 _w_2)))

(fn `ConvertFloatArrayTo1Vector`
  (params (floats :type "Array of Float (double-precision)"))
  (returns (vectors :type "Vector Structure"))
  (if (> (`KismetArrayLibrary.Array_Length` floats) 2)
    (return (`KismetMathLibrary.MakeVector` (`|GetArrayItem` floats) (`|GetArrayItem` floats 1) (`|GetArrayItem` floats 2)))))

(fn `ConvertFloatArrayToPositionVector`
  (params (floats :type "Array of Float (double-precision)"))
  (returns (vectors :type "Array of Vector Structure"))
  (locals (myvectors :type "Array of Vector Structure") (counter :type Integer) (counterOfVectors :type Integer))
  (bind _myvectors (`local.myvectors`))
  (bind _counter (`local.counter`))
  (`KismetArrayLibrary.Array_Clear` _myvectors)
  (for _index (range (+ (`KismetArrayLibrary.Array_Length` floats) 1))
    (if (== (`local.counter`) _index)
      (if (`KismetArrayLibrary.Array_Contains` (`self.jointFilter`) (`local.counterOfVectors`))
        (`KismetArrayLibrary.Array_Add` _myvectors (`KismetMathLibrary.MakeVector` (* (`|GetArrayItem` floats _counter) -100) (* (`|GetArrayItem` floats (+ _counter 1)) -100) (* (`|GetArrayItem` floats (+ _counter 2)) -100))))
      (set `local.counter` (+ _index 3))
      (set `local.counterOfVectors` (+ (`local.counterOfVectors`) 1))))
  (return _myvectors))

(fn `ConvertFloatArrayToRotator`
  (params (floats :type "Array of Float (double-precision)"))
  (returns (vectors :type "Array of Vector4 Structure"))
  (locals (myvectors :type "Array of Vector4 Structure") (counter :type Integer) (insideQuatCounter :type Integer) (counterCorrespondingToFilter :type Integer))
  (bind _myvectors (`local.myvectors`))
  (bind _counter (`local.counter`))
  (`KismetArrayLibrary.Array_Clear` _myvectors)
  (for _index (range (+ (`KismetArrayLibrary.Array_Length` floats) 1))
    (if (== (`local.counter`) _index)
      (if (`KismetArrayLibrary.Array_Contains` (`self.jointFilter`) (`local.insideQuatCounter`))
        (bind _rotationsadapted (`self.Adapt RotationsBlueprint` (`KismetMathLibrary.MakeVector4` (`|GetArrayItem` floats (+ _counter 1)) (`|GetArrayItem` floats (+ _counter 2)) (`|GetArrayItem` floats (+ _counter 3)) (`|GetArrayItem` floats _counter)) (`local.counterCorrespondingToFilter`)))
        (set `local.counterCorrespondingToFilter` (+ (`local.counterCorrespondingToFilter`) 1))
        (`KismetArrayLibrary.Array_Add` _myvectors _rotationsadapted))
      (set `local.counter` (+ _index 4))
      (set `local.insideQuatCounter` (+ (`local.insideQuatCounter`) 1))))
  (return _myvectors))

(fn `CreateEdges`
  (locals (parent :type Integer) (child :type Integer))
  (set `local.parent` 1000)
  (for _array_element (`self.jointConnectivity`)
    (if (== _array_element 1000)
      (set `local.parent` 1000)
      (elif (== (`local.parent`) 1000)
        (set `local.parent` _array_element)
        (else
          (`KismetArrayLibrary.Array_Add` (`self.edges`) (make `/Game/Pedro/MyEdges` "0.000000,0.000000,0.000000|0.000000,0.000000,0.000000|1.000000,1.000000,1.000000" 0.0 (`local.parent`) _array_element))
          (set `local.parent` _array_element))))))

(fn `DefaultStatement`
  (params (Address :type "OSCAddress Structure (by ref)"))
  (bind _returnvalue (`OSCManager.GetOSCAddressFullPath` Address))
  (if (not (`KismetArrayLibrary.Array_Contains` (`self.debugStrings`) _returnvalue))
    (`KismetArrayLibrary.Array_Add` (`self.debugStrings`) _returnvalue)
    (`KismetSystemLibrary.PrintString` (`KismetStringLibrary.Concat_StrStr` "There is no acction set for this address: " _returnvalue) true true (struct :`G` 0.66 :`B` 1.0 :`A` 1.0) 2000.0)))

(fn `Set Material Float`
  (params (Array :type "Array of Float (single-precision)") (`Name Material Parameter` :type Name))
  (bind _returnvalue (`KismetArrayLibrary.Array_Length` Array))
  (`KismetSystemLibrary.PrintString` (`KismetStringLibrary.Conv_IntToString` _returnvalue))
  (if (> _returnvalue 0)
    (`MaterialInstanceDynamic.SetScalarParameterValue` (`self.RaymarchingMat`) `Name Material Parameter` (`|GetArrayItem` Array))))

(fn `SetMaterialColorParameter`
  (params (floats :type "Array of Float (double-precision) (by ref)") (nameMaterialParameter :type Name))
  (bind _vectors (`self.ConvertFloatArrayTo1Vector` floats))
  (`MaterialInstanceDynamic.SetVectorParameterValue` (`self.RaymarchingMat`) nameMaterialParameter (`KismetMathLibrary.MakeColor` (.x _vectors) (.y _vectors) (.z _vectors))))

(fn `UserConstructionScript`)