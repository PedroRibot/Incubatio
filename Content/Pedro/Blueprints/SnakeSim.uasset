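; SnakeSim is an actor that simulates a snake as a chain of spawned joint actors trailing it.
; BeginPlay spawns the joints along X and starts a looping timer at a configurable Fps, leaving Tick empty.
; Each step moves the actor back and forth between two hardcoded points.
; Joints farther than the spacing interpolate position and look-at rotation toward their predecessor, more slowly down the chain; the sideways wave offset is unconnected.
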(event `self.ReceiveBeginPlay`
  (`|ExecutionSequence`
    (:`then_0`
      (for _index (range (`self.SnakeLong`))
        (bind _returnvalue (`|SpawnActorFromClass` "/Game/Pedro/Blueprints/Debug/SnakeJoints.SnakeJoints_C" (`KismetMathLibrary.MakeTransform` (`KismetMathLibrary.MakeVector` (`KismetMathLibrary.Conv_IntToDouble` (* _index (`self.DiistanceBetween`))))) "Undefined" "MultiplyWithRoot" null null))
        (`KismetArrayLibrary.Array_Add` (`self.MyJoints`) _returnvalue)))
    (:`then_1`
      (`KismetSystemLibrary.K2_SetTimerDelegate` (delegate `MainLoop`) (/ 1.0 (`self.Fps`)) true))))

(event `MainLoop`
  (bind _myjoints (`self.MyJoints`))
  (bind _head_goint_to (`self.head_goint_to`))
  (bind _returnvalue (/ 1.0 (`self.Fps`)))
  (for (_array_element _array_index) _myjoints
    (if (!= _array_index 0)
      (`self.MoveAndLookWithInterpolation` _returnvalue _array_index _array_element (`|GetArrayItem` _myjoints (- _array_index 1)))
      (else
        (`self.MoveAndLookWithInterpolation` _returnvalue 0 _array_element self)
        (if (< (`KismetMathLibrary.Vector_Distance` _head_goint_to (`self.K2_GetActorLocation` self)) 10.0)
          ;[1 1 1] SHITTY AUTOMATIC
          (if (== (.x _head_goint_to) 1000.0)
            (set `self.head_goint_to` (-1000.0 0.0 0.0))
            (else
              (set `self.head_goint_to` (1000.0 0.0 0.0))))
          (else
            (`self.K2_SetActorLocation` (+ (* (`KismetMathLibrary.Normal` (- (`self.head_goint_to`) (`self.K2_GetActorLocation` self))) (`self.speed`) _returnvalue) (`self.K2_GetActorLocation` self)))))))))

(event `self.ReceiveTick`
  (params (DeltaSeconds :type "Float (single-precision)")))

(fn `MoveAndLookWithInterpolation`
  (params (DeltaTime :type "Float (single-precision)") (Index :type Integer) (actorToMove :type "Actor Object Reference") (actorTarget :type "Actor Object Reference"))
  (bind _returnvalue (`self.K2_GetActorLocation` actorTarget))
  (bind _returnvalue_2 (`self.K2_GetActorLocation` actorToMove))
  (bind _returnvalue_3 (`KismetMathLibrary.FMax` (- (`self.InterpolationSpeed`) Index) 2.0))
  (if (> (`KismetMathLibrary.Vector_Distance` _returnvalue_2 _returnvalue) (`self.DiistanceBetween`))
    (`self.K2_SetActorTransform` actorToMove (`KismetMathLibrary.MakeTransform` (`KismetMathLibrary.VInterpTo` _returnvalue_2 _returnvalue DeltaTime _returnvalue_3) (`KismetMathLibrary.RInterpTo` (`self.K2_GetActorRotation` actorToMove) (`KismetMathLibrary.FindLookAtRotation` _returnvalue_2 _returnvalue) DeltaTime _returnvalue_3)) false false)))

(fn `UserConstructionScript`)